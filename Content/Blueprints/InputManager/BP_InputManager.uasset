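; Input manager actor that registers itself as a receiver of Arduino BLE input.
; One tick after BeginPlay it finds the ArduinoBLEInputParser in the level, caches it and joins its receive-input object list, then leaves that list when destroyed.
; Its AccelerationInput function simply returns Up, with no processing of input in this graph.
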(event `self.ReceiveBeginPlay`
  (`KismetSystemLibrary.DelayUntilNextTick`)
  (bind _returnvalue (`GameplayStatics.GetActorOfClass` "/Script/VoodooManagement.ArduinoBLEInputParser"))
  (bind _output_get (set `self.ArdunioBLEInputParser` _returnvalue))
  (`ArduinoBLEInputParser.AddToReceiveInputObjectList` _output_get self))

(event `self.ReceiveDestroyed`
  (`ArduinoBLEInputParser.RemoveFromReceiveObjectInputList` (`self.ArdunioBLEInputParser`) self))

(fn `AccelerationInput`
  (returns (Type :type "EMotionType Enum"))
  (return "up"))

(fn `UserConstructionScript`)