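; Gameplay input manager for a voodoo-themed office level where the player controls employees' behavior and productivity.
; BeginPlay applies the picked item's perk, starts music, camera and timer widget, and maps employees by ID.
; RFID selects an employee for the mini-camera, five buttons pin states on them, and cooldown-limited sound input yells at all employees.
; Tick totals productivity minus prior KPI, firing one-shot music stingers at thresholds.
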(event `self.ReceiveTick`
  (params (DeltaSeconds :type "Float (single-precision)"))
  (bind _values (`BlueprintMapLibrary.Map_Values` (`self.AllEmployees`)))
  (set `self.LevelTotalKPI` 0)
  (for _array_element _values
    (set `self.LevelTotalKPI` (+ (`self.LevelTotalKPI`) (`/Game/Blueprints/BP_TESTING.ProductivityScore` _array_element))))
  (bind _output_get (set `self.LevelTotalKPI` (- (`self.LevelTotalKPI`) (`self.PreviousLevelTotalKPI`))))
  (if (== _output_get 200)
    (`/Engine/EditorBlueprintResources/StandardMacros.DoOnce` false
      (:`Completed`
        (bind _returnvalue (`AddComponent|NODE_AddAudioComponent-3`))
        ;[1 1 1] Stinger 2
        (`AudioParameterControllerInterface.SetTriggerParameter` _returnvalue "Stop1")
        (`AudioParameterControllerInterface.SetTriggerParameter` _returnvalue "StartWav2")))
    (elif (> _output_get 100)
      (`/Engine/EditorBlueprintResources/StandardMacros.DoOnce` false
        (:`Completed`
          (bind _returnvalue_2 (`AddComponent|NODE_AddAudioComponent-2`))
          (`AudioParameterControllerInterface.SetTriggerParameter` _returnvalue_2 "Stop0")
          ;[1 1 1] Stinger 1
          (`AudioParameterControllerInterface.SetTriggerParameter` _returnvalue_2 "StartWav1"))))))

(event `self.ReceiveBeginPlay`
  (`parent.ReceiveBeginPlay`)
  (`|ExecutionSequence`
    (:`then_0`
      (bind _asgi_third_person_game_instance (cast `/Game/Blueprints/GI_ThirdPersonGameInstance` (`GameplayStatics.GetGameInstance`)))
      (`self.ActivateItem` (`/Game/Blueprints/GI_ThirdPersonGameInstance.PickingItem` _asgi_third_person_game_instance)))
    (:`then_1`
      (`GameplayStatics.PlaySound2D` "/Game/Audio/Music/VoodooMusicSystem.VoodooMusicSystem" 1.0 1.0 0.0 null null)
      (`PlayerController.SetViewTargetWithBlend` (`GameplayStatics.GetPlayerController` 0) (`self.CameraActor`) 0.0 "VTBlend_Linear" 0.0 false))
    (:`then_2`
      (bind _returnvalue (`|CreateWidget` "/Game/UI/BPW_Timer.BPW_Timer_C"))
      (`UserWidget.AddToViewport` _returnvalue 0)
      (set `/Game/UI/BPW_Timer.MinuteInterval` (`self.MinuteInterval`) _returnvalue)
      (set `/Game/UI/BPW_Timer.TargetMinute` (`self.TargetMinute`) _returnvalue)
      (set `/Game/UI/BPW_Timer.CurrentMinute` (`self.StartingMinute`) _returnvalue)
      (`/Game/UI/BPW_Timer.BeginCountingDown` _returnvalue))
    (:`then_3`
      (bind _outactors (`GameplayStatics.GetAllActorsOfClass` "/Game/Blueprints/BP_TESTING.BP_TESTING_C"))
      (if (`KismetArrayLibrary.Array_IsNotEmpty` _outactors)
        (`self.SetChoosingActor` (2.0 2.0 2.0) (`|GetArrayItem` _outactors))
        (for _array_element _outactors
          (`BlueprintMapLibrary.Map_Add` (`self.AllEmployees`) (`/Game/Blueprints/BP_TESTING.ID` _array_element) _array_element)
          (bind _asgi_third_person_game_instance_2 (cast `/Game/Blueprints/GI_ThirdPersonGameInstance` (`GameplayStatics.GetGameInstance`)))
          (set `self.PreviousLevelTotalKPI` (`/Game/Blueprints/GI_ThirdPersonGameInstance.TotalKPI` _asgi_third_person_game_instance_2)))))))

(event `ArduinoBLEInputInterface.Button1Input`
  (`GameplayStatics.PlaySound2D` "/Game/Audio/Stab.Stab" 1.0 1.0 0.0 null null)
  (`self.PunchingActor` "NewEnumerator4" (`self.CurrentActor`))
  (`KismetSystemLibrary.PrintString` "BathRoomBreak"))

(event `ArduinoBLEInputInterface.Button2Input`
  (`GameplayStatics.PlaySound2D` "/Game/Audio/Stab.Stab" 1.0 1.0 0.0 null null)
  (`self.PunchingActor` "NewEnumerator3" (`self.CurrentActor`))
  (`KismetSystemLibrary.PrintString` "PlayingCellPhone"))

(event `ArduinoBLEInputInterface.Button3Input`
  (`GameplayStatics.PlaySound2D` "/Game/Audio/Stab.Stab" 1.0 1.0 0.0 null null)
  (`self.PunchingActor` "NewEnumerator2" (`self.CurrentActor`))
  (`KismetSystemLibrary.PrintString` "Sleeping"))

(event `ArduinoBLEInputInterface.Button4Input`
  (`GameplayStatics.PlaySound2D` "/Game/Audio/Stab.Stab" 1.0 1.0 0.0 null null)
  (`self.PunchingActor` "NewEnumerator5" (`self.CurrentActor`))
  (`KismetSystemLibrary.PrintString` "Hunger"))

(event `ArduinoBLEInputInterface.Button5Input`
  (`GameplayStatics.PlaySound2D` "/Game/Audio/Stab.Stab" 1.0 1.0 0.0 null null)
  (`self.PunchingActor` "NewEnumerator7" (`self.CurrentActor`))
  (`KismetSystemLibrary.PrintString` "TrashTalk"))

(event `ArduinoBLEInputInterface.RFIDInput`
  (params (ID :type String))
  (bind (_value _returnvalue) (`BlueprintMapLibrary.Map_Find` (`self.AllEmployees`) ID))
  (if _returnvalue
    (`self.MatchingRFID` _value)))

(event `SetYellingIsReady`
  (set `self.IsYellingReady` true))

(event `ArduinoBLEInputInterface.SoundInput`
  (if (`self.IsYellingReady`)
    (set `self.IsYellingReady` false)
    (`KismetSystemLibrary.PrintString` "Yelling")
    (bind _outactors (`GameplayStatics.GetAllActorsOfClass` "/Game/Blueprints/BP_TESTING.BP_TESTING_C"))
    (for _array_element _outactors
      (if (`/Game/Blueprints/BP_TESTING.StateCanBeChanged` _array_element)
        (`/Game/Blueprints/BP_TESTING.GetBackToWork` _array_element)
        (else
          (bind _returnvalue (`AIBlueprintHelperLibrary.GetBlackboard` _array_element))
          (`BlackboardComponent.SetValueAsFloat` _returnvalue "BathRoomTime" 0.0)
          (`BlackboardComponent.SetValueAsBool` _returnvalue "IsInBathRoom" true)
          (set `/Game/Blueprints/BP_TESTING.CurrentState` "NewEnumerator4" _array_element))))
    (`KismetSystemLibrary.K2_SetTimerDelegate` (delegate `SetYellingIsReady`) (`self.YellingCoolDown`))))

(event `StoreEmployeeKIP`)

(fn `ActivateItem`
  (params (test :type Integer :default -1))
  (switch `int` test
    (:`0`
      (`KismetSystemLibrary.PrintString` "Ritual Drums")
      (bind _outactors (`GameplayStatics.GetAllActorsOfClass` "/Game/Blueprints/BP_TESTING.BP_TESTING_C"))
      (for _array_element _outactors
        (set `/Game/Blueprints/BP_TESTING.ProductivityIncreaseRate` (* (`/Game/Blueprints/BP_TESTING.ProductivityIncreaseRate` _array_element) 3) _array_element)))
    (:`1`
      (`KismetSystemLibrary.PrintString` "Asson")
      (set `self.YellingCoolDown` 5.0))
    (:`2`
      (`KismetSystemLibrary.PrintString` "Protective Charm")
      (bind _returnvalue (`GameplayStatics.GetActorOfClass` "/Game/Blueprints/BP_Item.BP_Item_C"))
      (set `/Game/Blueprints/BP_Item.ProtectiveLeft` 4 _returnvalue))
    (:`3`
      (`KismetSystemLibrary.PrintString` "Veve of Baron Samedi")
      (bind _outactors_2 (`GameplayStatics.GetAllActorsOfClass` "/Game/Blueprints/BP_TESTING.BP_TESTING_C"))
      (bind _output (`|GetArrayItem` _outactors_2 (`KismetMathLibrary.RandomInteger` (`KismetArrayLibrary.Array_Length` _outactors_2))))
      (set `/Game/Blueprints/BP_TESTING.IsAPerfectEmployee` true _output)
      (`KismetSystemLibrary.PrintString` (`KismetSystemLibrary.GetDisplayName` _output)))))

(fn `ClearCircle`
  (params (NewParam :type "/Game/Blueprints/BP_TESTING Object Reference"))
  (`/Game/Blueprints/BP_TESTING.SetCircle` NewParam (0.0 0.0 0.0)))

(fn `MatchingRFID`
  (params (NewParam :type "/Game/Blueprints/BP_TESTING Object Reference"))
  (`self.ClearCircle` (`self.CurrentActor`))
  (`self.ResetCameraFocus`)
  (`self.SetChoosingActor` (2.0 2.0 2.0) NewParam))

(fn `NewFunction`)

(fn `PunchingActor`
  (params (EmployeeState :type "/Game/EmployeeStates Enum" :default "NewEnumerator0") (Target :type "/Game/Blueprints/BP_TESTING Object Reference"))
  (`/Game/Blueprints/BP_TESTING.Pined` Target EmployeeState))

(fn `ResetCameraFocus`
  (set `SceneCaptureComponent2D.TextureTarget` null (`/Game/Blueprints/BP_TESTING.SceneCaptureComponent2D` (`self.CurrentActor`))))

(fn `SetChoosingActor`
  (params (CircleScale :type "Vector Structure") (Target :type "/Game/Blueprints/BP_TESTING Object Reference"))
  (`/Game/Blueprints/BP_TESTING.SetCircle` Target CircleScale)
  (bind _output_get (set `self.CurrentActor` Target))
  (set `SceneCaptureComponent2D.TextureTarget` "/Game/Materials/miniCameraTarget.miniCameraTarget" (`/Game/Blueprints/BP_TESTING.SceneCaptureComponent2D` _output_get)))

(fn `UserConstructionScript`
  (`parent.UserConstructionScript`))