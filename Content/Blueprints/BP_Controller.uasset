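; BP_Controller manages stage progression through a list of streamed levels, moving to the next, previous or current stage.
; Bounds-checked events call three identical GoToLevel macros that clear all widgets, unload the current stream level, update CurrentStage and load the target, blocking on unload and load.
; TimeIsUp has the GI_ThirdPersonGameInstance calculate and save the total KPI, then advances to the next stage.
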(event `GoToNextLevel`
  (bind _returnvalue (+ (`self.CurrentStage`) 1))
  (if (> (`KismetArrayLibrary.Array_Length` (`self.LevelList`)) _returnvalue)
    (`WidgetLayoutLibrary.RemoveAllWidgets`)
    (`GameplayStatics.UnloadStreamLevelBySoftObjectPtr` (`|GetArrayItem` (`self.LevelList`) (`self.CurrentStage`)) true)
    (bind _output_get (set `self.CurrentStage` _returnvalue))
    (`GameplayStatics.LoadStreamLevelBySoftObjectPtr` (`|GetArrayItem` (`self.LevelList`) _output_get) true true)))

(event `RestartCurrentLevel`
  (`WidgetLayoutLibrary.RemoveAllWidgets`)
  (`GameplayStatics.UnloadStreamLevelBySoftObjectPtr` (`|GetArrayItem` (`self.LevelList`) (`self.CurrentStage`)) true)
  (bind _output_get (set `self.CurrentStage` (`self.CurrentStage`)))
  (`GameplayStatics.LoadStreamLevelBySoftObjectPtr` (`|GetArrayItem` (`self.LevelList`) _output_get) true true))

(event `GoToFormerLevel`
  (bind _returnvalue (- (`self.CurrentStage`) 1))
  (if (>= _returnvalue 0)
    (`WidgetLayoutLibrary.RemoveAllWidgets`)
    (`GameplayStatics.UnloadStreamLevelBySoftObjectPtr` (`|GetArrayItem` (`self.LevelList`) (`self.CurrentStage`)) true)
    (bind _output_get (set `self.CurrentStage` _returnvalue))
    (`GameplayStatics.LoadStreamLevelBySoftObjectPtr` (`|GetArrayItem` (`self.LevelList`) _output_get) true true)))

(event `TimeIsUp`
  (bind _asgi_third_person_game_instance (cast `/Game/Blueprints/GI_ThirdPersonGameInstance` (`GameplayStatics.GetGameInstance`)))
  (`/Game/Blueprints/GI_ThirdPersonGameInstance.CalculateAndSaveTotalKPI` _asgi_third_person_game_instance)
  (`self.GoToNextLevel`))

(fn `UserConstructionScript`)