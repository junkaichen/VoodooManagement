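; Debug actor that simulates Arduino BLE controller input with Enhanced Input keys, standing in for the physical hardware.
; On BeginPlay it adds a debug mapping context and finds the ArduinoBLEInputParser, caching its UID-to-name list.
; Button, shout and character-switch keys forward messages to every object in the parser's receive list, the switch cycling names as fake RFID reads.
; Level keys call next, former or restart on BP_Controller.
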(event `self.ReceiveBeginPlay`
  (bind _returnvalue (`GameplayStatics.GetPlayerController` 0))
  (`self.EnableInput` _returnvalue)
  (`EnhancedInputSubsystemInterface.AddMappingContext` (pcsubsystem `EnhancedInputLocalPlayerSubsystem` _returnvalue) "/Game/Input/DebugInputMappingContext.DebugInputMappingContext" 0 (make `ModifyContextOptions` true))
  (`KismetSystemLibrary.DelayUntilNextTick`)
  (bind _returnvalue_2 (`GameplayStatics.GetActorOfClass` "/Script/VoodooManagement.ArduinoBLEInputParser"))
  (bind _output_get (set `self.BLEParser` _returnvalue_2))
  (`/Engine/EditorBlueprintResources/StandardMacros.IsValid` _output_get
    (:`Is Valid`
      (bind _values (`BlueprintMapLibrary.Map_Values` (`ArduinoBLEInputParser.UIDToNameMap` _output_get)))
      (set `self.NameList` _values))))

(event `EnhancedInput|/Game/Input/IA_Button1`
  (params (ActionValue :type Boolean) (ElapsedSeconds :type "Float (double-precision)") (TriggeredSeconds :type "Float (double-precision)") (InputAction :type "InputAction Object Reference" :default "/Game/Input/IA_Button1.IA_Button1"))
  (bind _bleparser (`self.BLEParser`))
  (:`Started`
    (bind _result (`BlueprintSetLibrary.Set_ToArray` (`ArduinoBLEInputParser.ReceiveInputObjectList` _bleparser)))
    (for _array_element _result
      (message `ArduinoBLEInputInterface.Button1Input` _array_element)
      (`ArduinoBLEInputParser.MotorVibrate` _bleparser 0))))

(event `EnhancedInput|/Game/Input/IA_Button2`
  (params (ActionValue :type Boolean) (ElapsedSeconds :type "Float (double-precision)") (TriggeredSeconds :type "Float (double-precision)") (InputAction :type "InputAction Object Reference" :default "/Game/Input/IA_Button2.IA_Button2"))
  (:`Started`
    (bind _result (`BlueprintSetLibrary.Set_ToArray` (`ArduinoBLEInputParser.ReceiveInputObjectList` (`self.BLEParser`))))
    (for _array_element _result
      (message `ArduinoBLEInputInterface.Button2Input` _array_element))))

(event `EnhancedInput|/Game/Input/IA_Button3`
  (params (ActionValue :type Boolean) (ElapsedSeconds :type "Float (double-precision)") (TriggeredSeconds :type "Float (double-precision)") (InputAction :type "InputAction Object Reference" :default "/Game/Input/IA_Button3.IA_Button3"))
  (:`Started`
    (bind _result (`BlueprintSetLibrary.Set_ToArray` (`ArduinoBLEInputParser.ReceiveInputObjectList` (`self.BLEParser`))))
    (for _array_element _result
      (message `ArduinoBLEInputInterface.Button3Input` _array_element))))

(event `EnhancedInput|/Game/Input/IA_Button4`
  (params (ActionValue :type Boolean) (ElapsedSeconds :type "Float (double-precision)") (TriggeredSeconds :type "Float (double-precision)") (InputAction :type "InputAction Object Reference" :default "/Game/Input/IA_Button4.IA_Button4"))
  (:`Started`
    (bind _result (`BlueprintSetLibrary.Set_ToArray` (`ArduinoBLEInputParser.ReceiveInputObjectList` (`self.BLEParser`))))
    (for _array_element _result
      (message `ArduinoBLEInputInterface.Button4Input` _array_element))))

(event `EnhancedInput|/Game/Input/IA_Button5`
  (params (ActionValue :type Boolean) (ElapsedSeconds :type "Float (double-precision)") (TriggeredSeconds :type "Float (double-precision)") (InputAction :type "InputAction Object Reference" :default "/Game/Input/IA_Button5.IA_Button5"))
  (:`Started`
    (bind _result (`BlueprintSetLibrary.Set_ToArray` (`ArduinoBLEInputParser.ReceiveInputObjectList` (`self.BLEParser`))))
    (for _array_element _result
      (message `ArduinoBLEInputInterface.Button5Input` _array_element))))

(event `EnhancedInput|/Game/Input/IA_Shout`
  (params (ActionValue :type Boolean) (ElapsedSeconds :type "Float (double-precision)") (TriggeredSeconds :type "Float (double-precision)") (InputAction :type "InputAction Object Reference" :default "/Game/Input/IA_Shout.IA_Shout"))
  (:`Started`
    (bind _result (`BlueprintSetLibrary.Set_ToArray` (`ArduinoBLEInputParser.ReceiveInputObjectList` (`self.BLEParser`))))
    (for _array_element _result
      (message `ArduinoBLEInputInterface.SoundInput` _array_element))))

(event `EnhancedInput|/Game/Input/IA_SwitchCharacter`
  (params (ActionValue :type "Float (double-precision)") (ElapsedSeconds :type "Float (double-precision)") (TriggeredSeconds :type "Float (double-precision)") (InputAction :type "InputAction Object Reference" :default "/Game/Input/IA_SwitchCharacter.IA_SwitchCharacter"))
  (bind _namelist (`self.NameList`))
  (bind _returnvalue (`KismetArrayLibrary.Array_Length` _namelist))
  (:`Started`
    (bind _output_get (set `self.CurentNameIndex` (`KismetMathLibrary.SelectInt` (mod (+ (`self.CurentNameIndex`) 1) _returnvalue) (mod (+ (`self.CurentNameIndex`) (- _returnvalue 1)) _returnvalue) (> ActionValue 0.0))))
    (bind _result (`BlueprintSetLibrary.Set_ToArray` (`ArduinoBLEInputParser.ReceiveInputObjectList` (`self.BLEParser`))))
    (for _array_element _result
      (message `ArduinoBLEInputInterface.RFIDInput` _array_element (`|GetArrayItem` _namelist _output_get)))))

(event `EnhancedInput|/Game/Input/IA_NextLevel`
  (params (ActionValue :type Boolean) (ElapsedSeconds :type "Float (double-precision)") (TriggeredSeconds :type "Float (double-precision)") (InputAction :type "InputAction Object Reference" :default "/Game/Input/IA_NextLevel.IA_NextLevel"))
  (:`Started`
    (bind _asbp_controller (cast `/Game/Blueprints/BP_Controller` (`GameplayStatics.GetPlayerController` 0)))
    (`/Game/Blueprints/BP_Controller.GoToNextLevel` _asbp_controller)))

(event `EnhancedInput|/Game/Input/IA_RestartLevel`
  (params (ActionValue :type Boolean) (ElapsedSeconds :type "Float (double-precision)") (TriggeredSeconds :type "Float (double-precision)") (InputAction :type "InputAction Object Reference" :default "/Game/Input/IA_RestartLevel.IA_RestartLevel"))
  (:`Started`
    (bind _asbp_controller (cast `/Game/Blueprints/BP_Controller` (`GameplayStatics.GetPlayerController` 0)))
    (`/Game/Blueprints/BP_Controller.RestartCurrentLevel` _asbp_controller)))

(event `EnhancedInput|/Game/Input/IA_FormerLevel`
  (params (ActionValue :type Boolean) (ElapsedSeconds :type "Float (double-precision)") (TriggeredSeconds :type "Float (double-precision)") (InputAction :type "InputAction Object Reference" :default "/Game/Input/IA_FormerLevel.IA_FormerLevel"))
  (:`Started`
    (bind _asbp_controller (cast `/Game/Blueprints/BP_Controller` (`GameplayStatics.GetPlayerController` 0)))
    (`/Game/Blueprints/BP_Controller.GoToFormerLevel` _asbp_controller)))

(fn `UserConstructionScript`)