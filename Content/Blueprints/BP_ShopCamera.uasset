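; Shop camera for the item-picking stage, driven by Arduino BLE button input.
; Buttons 1-4 zoom from the origin to that item's BPCamLocation path point via timeline lerp, then show the picking widget; Button 5 backs out.
; Pressing the same button again saves the pick to the GameInstance, swaps streamed Level_2 for Level_3 and starts gameplay on the controller.
; Before stage 2, Button 2 clears widgets and enters it.
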(event `self.ReceiveBeginPlay`
  (`KismetSystemLibrary.DelayUntilNextTick`)
  (bind _returnvalue (`GameplayStatics.GetActorOfClass` "/Script/VoodooManagement.ArduinoBLEInputParser"))
  (bind _output_get (set `self.ArdunioBLEInputParser` _returnvalue))
  (`ArduinoBLEInputParser.AddToReceiveInputObjectList` _output_get self)
  (set `self.ItemLocation` (`/Game/Blueprints/BP_WalkPath.WalkPathPoint` (`self.BP_CamLocation`)))
  (set `self.OriginPoint` (`self.K2_GetActorLocation`))
  (set `self.NewVar` (`self.GetTransform`)))

(event `self.ReceiveDestroyed`
  (`ArduinoBLEInputParser.RemoveFromReceiveObjectInputList` (`self.ArdunioBLEInputParser`) self))

(event `ArduinoBLEInputInterface.Button1Input`
  (if (== (`self.Stage`) 2)
    (set `self.NewPicking` 0)
    (if (== (`self.CurrentPicking`) -1) :!label _label
      (set `self.CurrentPicking` (`self.NewPicking`))
      (bind (_direction _zoomintime) (`Timeline|CameraZoomIn` :!via `PlayFromStart`)
        (:`Update`
          (`self.ZoomIn` _zoomintime (`self.CurrentPicking`)))
        (:`Finished`
          (bind _returnvalue (`|CreateWidget` "/Game/UI/BPW_PickingItem.BPW_PickingItem_C"))
          (bind _output_get (set `self.PickItemWidget` _returnvalue))
          (`UserWidget.AddToViewport` _output_get 0)))
      (elif (== (`self.CurrentPicking`) (`self.NewPicking`))
        (bind _asgi_third_person_game_instance (cast `/Game/Blueprints/GI_ThirdPersonGameInstance` (`GameplayStatics.GetGameInstance`)))
        (set `/Game/Blueprints/GI_ThirdPersonGameInstance.PickingItem` (`self.CurrentPicking`) _asgi_third_person_game_instance)
        (`WidgetLayoutLibrary.RemoveAllWidgets`)
        (`GameplayStatics.LoadStreamLevelBySoftObjectPtr` "/Game/ThirdPerson/Maps/Level_3.Level_3" true true)
        (bind _asbp_controller (cast `/Game/Blueprints/BP_Controller` (`GameplayStatics.GetPlayerController` 0)))
        (set `/Game/Blueprints/BP_Controller.CurrentStage` (+ (`/Game/Blueprints/BP_Controller.CurrentStage` _asbp_controller) 1) _asbp_controller)
        (set `/Game/Blueprints/BP_Controller.IsInGameplay` true _asbp_controller)
        (`GameplayStatics.UnloadStreamLevelBySoftObjectPtr` "/Game/Level/Level_2.Level_2" true)))))

(event `ArduinoBLEInputInterface.Button2Input`
  (if (== (`self.Stage`) 2)
    (set `self.NewPicking` 1)
    (goto _label)
    (else
      (set `self.Stage` 2)
      (`WidgetLayoutLibrary.RemoveAllWidgets`))))

(event `ArduinoBLEInputInterface.Button3Input`
  (if (== (`self.Stage`) 2)
    (set `self.NewPicking` 2)
    (goto _label)))

(event `ArduinoBLEInputInterface.Button4Input`
  (if (== (`self.Stage`) 2)
    (set `self.NewPicking` 3)
    (goto _label)))

(event `ArduinoBLEInputInterface.Button5Input`
  (if (== (`self.Stage`) 2)
    (bind _pickitemwidget (`self.PickItemWidget`)
      (:`then`
        (`Widget.RemoveFromParent` _pickitemwidget)
        (bind (_direction _zoomintime) (`Timeline|Timeline` :!via `PlayFromStart`)
          (:`Update`
            (`self.ZoomOut` _zoomintime (`self.CurrentPicking`)))
          (:`Finished`
            (set `self.CurrentPicking` -1))))
      (:`else`))))

(fn `AccelerationInput`
  (returns (Type :type "EMotionType Enum"))
  (return "up"))

(fn `UserConstructionScript`)

(fn `ZoomIn`
  (params (Alpha :type "Float (single-precision)") (ItemNum :type Integer))
  (`SceneComponent.K2_SetWorldLocation` (`self.DefaultSceneRoot`) (`KismetMathLibrary.VLerp` (`self.OriginPoint`) (`KismetMathLibrary.TransformLocation` (`self.GetTransform` (`self.BP_CamLocation`)) (`|GetArrayItem` (`self.ItemLocation`) ItemNum)) Alpha) false false))

(fn `ZoomOut`
  (params (Alpha :type "Float (single-precision)") (ItemNum :type Integer))
  (`SceneComponent.K2_SetWorldLocation` (`self.DefaultSceneRoot`) (`KismetMathLibrary.VLerp` (`KismetMathLibrary.TransformLocation` (`self.GetTransform` (`self.BP_CamLocation`)) (`|GetArrayItem` (`self.ItemLocation`) ItemNum)) (`self.OriginPoint`) Alpha) false false))