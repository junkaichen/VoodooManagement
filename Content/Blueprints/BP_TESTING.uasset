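; Office employee AI character that randomly switches between working, slacking states (sleep, hunger, phone, trash talk) and walking off to the bathroom or elsewhere.
; RandomState picks an enum state after a random delay, using timelines to slide chair and mesh, adding sounds, Niagara effects or props, and updating the Blackboard for roaming states.
; Working accrues a displayed productivity score, seeded from GameInstance KPI.
; Pined interrupts matching slacking or otherwise docks KPI, unless BP_Item protection absorbs it.
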(event `MoveChairForwardEvent`
  (bind _audio (`self.Audio`))
  ;[1 1 1] MoveChairForward
  (bind (_direction _movechairtime) (`Timeline|Timeline_6` :!via `PlayFromStart`)
    (:`Update`
      (if (not (`self.IsForward`))
        (`self.MoveChairFoward` _movechairtime)
        (`self.MoveEmployeeForward` _movechairtime)))
    (:`Finished`
      (set `self.IsForward` true)
      (`AudioComponent.SetSound` _audio "/Game/Audio/Unused/Keyboard_01.Keyboard_01")
      (`AudioComponent.Play` _audio 0.0))))

(event `self.ReceiveEndPlay`
  (params (EndPlayReason :type "EEndPlayReason Enum" :default "Destroyed"))
  (bind _ardurio (`self.Ardurio`))
  ;[1 1 1] GameEnd Close Arduino Portal
  (`/Engine/EditorBlueprintResources/StandardMacros.IsValid` _ardurio
    (:`Is Valid`
      (`SerialCom.Close` _ardurio))))

(event `self.ReceiveBeginPlay`
  (`self.Add Hair`)
  (bind _asgi_third_person_game_instance (cast `/Game/Blueprints/GI_ThirdPersonGameInstance` (`GameplayStatics.GetGameInstance`)))
  (bind (_value _returnvalue) (`BlueprintMapLibrary.Map_Find` (`/Game/Blueprints/GI_ThirdPersonGameInstance.EmployeeKPI` _asgi_third_person_game_instance) (`self.ID`)))
  (if _returnvalue
    _
    (else
      _))
  (set `self.ProductivityScore` _value)
  (if (not (`self.IsAPerfectEmployee`))
    (`self.RandomState`))
  (set `self.MeshStartTransform` (`SceneComponent.GetRelativeTransform` (`self.Mesh`)))
  (set `self.ChairPointPosition` (`SceneComponent.GetRelativeTransform` (`self.ChairPoint`))))

(event `RandomState`
  (bind _audio (`self.Audio`))
  (bind _audio_2 (`self.Audio`))
  (bind _audio_3 (`self.Audio`))
  (bind _audio_4 (`self.Audio`))
  (bind _audio_5 (`self.Audio`))
  (if (`self.StateCanBeChanged`)
    (`KismetSystemLibrary.Delay` (`KismetMathLibrary.RandomFloatInRange` 5.0 20.0))
    (`self.ResetStates`)
    (bind _output_get (set `self.TargetState` (cast `/Game/EmployeeStates` (`KismetMathLibrary.Conv_IntToByte` (`KismetMathLibrary.RandomIntegerInRange` 0 (enumcount `/Game/EmployeeStates`))))))
    (switch `/Game/EmployeeStates` _output_get
      (:`NewEnumerator0`
        ;[1 1 1] C_GoToBathroom
        (`AudioComponent.Stop` (`self.Audio`))
        (bind (_direction _movechairtime) (`Timeline|Timeline` :!via `PlayFromStart`)
          (:`Update`
            (if (`self.IsForward`)
              (`self.MoveChairBackward` _movechairtime)
              (`self.MoveEmployeeBackward` _movechairtime)))
          (:`Finished`
            (`SceneComponent.K2_SetRelativeTransform` (`self.Mesh`) (`self.ChairPointPosition`) false false)
            (`SceneComponent.K2_SetRelativeTransform` (`self.ChairPoint`) (`self.ChairPointPosition`) false false)
            (`SceneComponent.K2_SetRelativeTransform` (`self.Mesh`) (`self.MeshStartTransform`) false false)
            (`self.PlayAnimMontage` "/Game/Animations/AM_CBathRoomBreak.AM_CBathRoomBreak")
            (bind _output_get_2 (set `self.CurrentState` (`self.TargetState`)))
            (`BlackboardComponent.SetValueAsEnum` (`AIBlueprintHelperLibrary.GetBlackboard` null) "CurrentState" _output_get_2)
            (set `self.IsForward` false)
            (set `self.StateCanBeChanged` false)
            (`self.RandomState`))))
      (:`NewEnumerator2`
        ;[1 1 1] Sleeping
        (bind (_direction_2 _movechairtime_2) (`Timeline|Timeline_3` :!via `PlayFromStart`)
          (:`Update`
            (if (`self.IsForward`)
              (`self.MoveChairBackward` _movechairtime_2)
              (`self.MoveEmployeeBackward` _movechairtime_2)))
          (:`Finished`
            (set `self.IsForward` false)
            (`AudioComponent.SetSound` _audio_4 "/Game/Audio/Snore.Snore")
            (`AudioComponent.Play` _audio_4 0.0)
            (`SceneComponent.SetHiddenInGame` (`self.Niagara`) false false)
            (`NiagaraComponent.SetAsset` (`self.Niagara`) "/Game/Animations/anima_VFX/N_Zsleep.N_Zsleep" true)
            (set `self.CurrentState` (`self.TargetState`) :!label _label)
            (`self.RandomState`))))
      (:`NewEnumerator1`
        ;[1 1 1] Working
        (bind (_direction_3 _movechairtime_3) (`Timeline|Timeline_4` :!via `PlayFromStart`)
          (:`Update`
            (if (not (`self.IsForward`))
              (`self.MoveChairFoward` _movechairtime_3)
              (`self.MoveEmployeeForward` _movechairtime_3)))
          (:`Finished`
            (set `self.IsForward` true)
            (`AudioComponent.SetSound` _audio_3 "/Game/Audio/Keyboard.Keyboard")
            (`AudioComponent.Play` _audio_3 0.0)
            (goto _label))))
      (:`NewEnumerator3`
        ;[1 1 1] PlayingCellPhone
        (bind (_direction_4 _movechairtime_4) (`Timeline|Timeline_0` :!via `PlayFromStart`)
          (:`Update`
            (if (`self.IsForward`)
              (`self.MoveChairBackward` _movechairtime_4)
              (`self.MoveEmployeeBackward` _movechairtime_4)))
          (:`Finished`
            (bind _returnvalue (`|SpawnActorFromClass` "/Game/Blueprints/AnimatedItems/BP_Phone.BP_Phone_C" (`KismetMathLibrary.MakeTransform` (0.0 0.0 0.0)) "Undefined" "OverrideRootScale" null self))
            (bind _output_get_3 (set `self.BP_Phone` _returnvalue))
            (`SceneComponent.K2_AttachToComponent` (`Actor.RootComponent` _output_get_3) (`self.Mesh`) "RightHandSocket" "KeepRelative" "KeepRelative" "KeepRelative" true)
            (set `self.IsForward` false)
            (`AudioComponent.SetSound` _audio_2 "/Game/Audio/PhoneTexting.PhoneTexting")
            (`AudioComponent.Play` _audio_2 0.0)
            (goto _label))))
      (:`NewEnumerator4`
        ;[1 1 1] C_GoToBathroom
        (`AudioComponent.Stop` (`self.Audio`))
        (bind (_direction_5 _movechairtime_5) (`Timeline|Timeline_8` :!via `PlayFromStart`)
          (:`Update`
            (if (`self.IsForward`)
              (`self.MoveChairBackward` _movechairtime_5)
              (`self.MoveEmployeeBackward` _movechairtime_5)))
          (:`Finished`
            (`SceneComponent.K2_SetRelativeTransform` (`self.Mesh`) (`self.ChairPointPosition`) false false)
            (`SceneComponent.K2_SetRelativeTransform` (`self.ChairPoint`) (`self.ChairPointPosition`) false false)
            (`SceneComponent.K2_SetRelativeTransform` (`self.Mesh`) (`self.MeshStartTransform`) false false)
            (bind _output_get_4 (set `self.CurrentState` (`self.TargetState`)))
            (`BlackboardComponent.SetValueAsEnum` (`AIBlueprintHelperLibrary.GetBlackboard` null) "CurrentState" _output_get_4)
            (set `self.IsForward` false)
            (set `self.StateCanBeChanged` false)
            (`self.RandomState`))))
      (:`NewEnumerator5`
        ;[1 1 1] Hunger
        (bind (_direction_6 _movechairtime_6) (`Timeline|Timeline_2` :!via `PlayFromStart`)
          (:`Update`
            (if (`self.IsForward`)
              (`self.MoveChairBackward` _movechairtime_6)
              (`self.MoveEmployeeBackward` _movechairtime_6)))
          (:`Finished`
            (set `self.IsForward` false)
            (`AudioComponent.SetSound` _audio_5 "/Game/Audio/Hungry.Hungry")
            (`AudioComponent.Play` _audio_5 0.0)
            (`SceneComponent.SetHiddenInGame` (`self.Niagara`) false false)
            (`NiagaraComponent.SetAsset` (`self.Niagara`) "/Game/Animations/anima_VFX/N_hunger.N_hunger" true)
            (goto _label))))
      (:`NewEnumerator7`
        (`AudioComponent.Stop` (`self.Audio`))
        ;[1 1 1] TrashTalking
        (`BlackboardComponent.SetValueAsVector` (`AIBlueprintHelperLibrary.GetBlackboard` null) "TargetLocation" (`self.K2_GetActorLocation` (`self.TrashTalkingPlace`)))
        (bind (_direction_7 _movechairtime_7) (`Timeline|Timeline_7` :!via `PlayFromStart`)
          (:`Update`
            (if (`self.IsForward`)
              (`self.MoveChairBackward` _movechairtime_7)
              (`self.MoveEmployeeBackward` _movechairtime_7)))
          (:`Finished`
            (`SceneComponent.K2_SetRelativeTransform` (`self.Mesh`) (`self.ChairPointPosition`) false false)
            (`SceneComponent.K2_SetRelativeTransform` (`self.ChairPoint`) (`self.ChairPointPosition`) false false)
            (`SceneComponent.K2_SetRelativeTransform` (`self.Mesh`) (`self.MeshStartTransform`) false false)
            (bind _output_get_5 (set `self.CurrentState` (`self.TargetState`)))
            (`BlackboardComponent.SetValueAsEnum` (`AIBlueprintHelperLibrary.GetBlackboard` null) "CurrentState" _output_get_5)
            (set `self.IsForward` false)
            (set `self.StateCanBeChanged` false)
            (`self.RandomState`))))
      (:`NewEnumerator8`
        ;[1 1 1] TrashTalking
        (`AudioComponent.Stop` (`self.Audio`))
        (`BlackboardComponent.SetValueAsVector` (`AIBlueprintHelperLibrary.GetBlackboard` null) "TargetLocation" (`self.K2_GetActorLocation` (`KismetArrayLibrary.Array_Random` (`self.CTrashTalkingPlace`))))
        (bind (_direction_8 _movechairtime_8) (`Timeline|Timeline_9` :!via `PlayFromStart`)
          (:`Update`
            (if (`self.IsForward`)
              (`self.MoveChairBackward` _movechairtime_8)
              (`self.MoveEmployeeBackward` _movechairtime_8)))
          (:`Finished`
            (`SceneComponent.K2_SetRelativeTransform` (`self.Mesh`) (`self.ChairPointPosition`) false false)
            (`SceneComponent.K2_SetRelativeTransform` (`self.ChairPoint`) (`self.ChairPointPosition`) false false)
            (`SceneComponent.K2_SetRelativeTransform` (`self.Mesh`) (`self.MeshStartTransform`) false false)
            (set `self.CurrentState` (`self.TargetState`))
            (`BlackboardComponent.SetValueAsEnum` (`AIBlueprintHelperLibrary.GetBlackboard` null) "CurrentState" (`self.CurrentState`))
            (set `self.IsForward` false)
            (set `self.StateCanBeChanged` false)
            (`self.RandomState`))))
      (:`NewEnumerator9`
        (bind (_direction_9 _movechairtime_9) (`Timeline|Timeline_10` :!via `PlayFromStart`)
          (:`Update`
            (if (`self.IsForward`)
              (`self.MoveChairBackward` _movechairtime_9)
              (`self.MoveEmployeeBackward` _movechairtime_9)))
          (:`Finished`
            (set `self.IsForward` false)
            (`AudioComponent.SetSound` _audio "/Game/Audio/Hungry.Hungry")
            (`AudioComponent.Play` _audio 0.0)
            (bind _returnvalue_2 (`|SpawnActorFromClass` "/Game/Blueprints/AnimatedItems/BP_Phone.BP_Phone_C" (`KismetMathLibrary.MakeTransform` (0.0 0.0 0.0)) "Undefined" "OverrideRootScale" null self))
            (bind _output_get_6 (set `self.BP_Phone` _returnvalue_2))
            (`SceneComponent.K2_AttachToComponent` (`Actor.RootComponent` _output_get_6) (`self.Mesh`) "RightHandSocket" "KeepRelative" "KeepRelative" "KeepRelative" true)
            (`/Game/Blueprints/BP_Computer.SwitchComputerOverloading` (`self.Computer`))
            (goto _label)))))
    (else
      (`KismetSystemLibrary.Delay` 0.5)
      (`self.RandomState`))))

(event `self.ReceiveTick`
  (params (DeltaSeconds :type "Float (single-precision)"))
  (if (`|EnumEquality` (`self.CurrentState`) "NewEnumerator1")
    (`KismetSystemLibrary.Delay` 0.3)
    (`self.UpdatingProductivityScore`)))

(event `Pined`
  (params (EmployeeState :type "/Game/EmployeeStates Enum" :default "NewEnumerator0"))
  (bind _returnvalue (`AIBlueprintHelperLibrary.GetBlackboard` null))
  (bind _returnvalue_2 (`AIBlueprintHelperLibrary.GetBlackboard` null))
  (if (`|EnumEquality` EmployeeState (`self.CurrentState`))
    (switch `/Game/EmployeeStates` EmployeeState
      (:`NewEnumerator2`
        (bind _output_get (set `self.CurrentState` "NewEnumerator1" :!label _label_2))
        (`BlackboardComponent.SetValueAsEnum` (`AIBlueprintHelperLibrary.GetBlackboard` null) "CurrentState" _output_get)
        (`self.MoveChairForwardEvent`)
        (`SceneComponent.SetHiddenInGame` (`self.Niagara`) true false))
      (:`NewEnumerator3`
        (goto _label_2))
      (:`NewEnumerator4`
        (if (== (`BlackboardComponent.GetValueAsInt` (`AIBlueprintHelperLibrary.GetBlackboard` null) "PatrolPointIndex") 0)
          (`self.DecreaseKPI` 10)
          (else
            (`BlackboardComponent.SetValueAsFloat` _returnvalue "BathRoomTime" 0.0)
            (`BlackboardComponent.SetValueAsBool` _returnvalue "IsInBathRoom" false)
            (`BlackboardComponent.SetValueAsBool` _returnvalue "IsInBathRoom" true))))
      (:`NewEnumerator5`
        (goto _label_2))
      (:`NewEnumerator7`
        (bind _output_get_2 (set `self.CurrentState` "NewEnumerator4"))
        (`BlackboardComponent.SetValueAsInt` _returnvalue_2 "PatrolPointIndex" 0)
        (`BlackboardComponent.SetValueAsEnum` _returnvalue_2 "CurrentState" _output_get_2)
        (`SceneComponent.SetHiddenInGame` (`self.Niagara`) true false)))
    (else
      (bind _returnvalue_3 (`GameplayStatics.GetActorOfClass` "/Game/Blueprints/BP_Item.BP_Item_C"))
      (if (`KismetSystemLibrary.IsValid` _returnvalue_3)
        (bind _protectiveleft (`/Game/Blueprints/BP_Item.ProtectiveLeft` _returnvalue_3))
        (if (> _protectiveleft 0)
          (set `/Game/Blueprints/BP_Item.ProtectiveLeft` (- _protectiveleft 1) _returnvalue_3)
          (else
            (if (`|EnumEquality` (`self.CurrentState`) "NewEnumerator1") :!label _label_3
              (`self.DecreaseKPI` 60)
              (else
                (`self.DecreaseKPI` 10)))))
        (else
          (goto _label_3))))))

(event `self.CapsuleComponent.OnComponentBeginOverlap`
  (params (OverlappedComponent :type "PrimitiveComponent Object Reference") (OtherActor :type "Actor Object Reference") (OtherComp :type "PrimitiveComponent Object Reference") (OtherBodyIndex :type Integer) (bFromSweep :type Boolean) (SweepResult :type "HitResult Structure (by ref)"))
  (bind _chair (`self.Chair`))
  (bind _chairpoint (`self.ChairPoint`))
  (bind _mesh (`self.Mesh`))
  (bind (_returnvalue_location _returnvalue_rotation) (`KismetMathLibrary.BreakTransform` (`SceneComponent.K2_GetComponentToWorld` (`/Game/Blueprints/BP_Chair.SitPosition` _chair))))
  (bind _asbp_chair (cast `/Game/Blueprints/BP_Chair` OtherActor))
  (if (== _asbp_chair _chair)
    (`SceneComponent.K2_SetWorldLocation` _chairpoint _returnvalue_location false false)
    (`SceneComponent.K2_SetWorldRotation` _chairpoint _returnvalue_rotation false false)
    (`SceneComponent.K2_SetWorldLocation` _mesh _returnvalue_location false false)
    (`SceneComponent.K2_SetWorldRotation` _mesh _returnvalue_rotation false false)
    (bind _output_get (set `self.CurrentState` "NewEnumerator1"))
    (`BlackboardComponent.SetValueAsEnum` (`AIBlueprintHelperLibrary.GetBlackboard` null) "CurrentState" _output_get)
    (`self.MoveChairForwardEvent`)
    (set `self.StateCanBeChanged` true)))

(fn `Add Hair`
  (bind _staticmesh (`self.StaticMesh`))
  (`StaticMeshComponent.SetStaticMesh` _staticmesh (`self.Hair_Mesh`))
  (`SceneComponent.K2_AttachToComponent` _staticmesh (`self.Mesh`) "hair" "SnapToTarget" "SnapToTarget" "SnapToTarget" true))

(fn `BackWardDesk`
  (params (Y :type "Float (single-precision)"))
  (bind (_returnvalue_location _returnvalue_rotation _returnvalue_scale) (`KismetMathLibrary.BreakTransform` (`SceneComponent.K2_GetComponentToWorld` (`self.Mesh`))))
  (`SceneComponent.K2_SetWorldTransform` (`self.Mesh`) (`KismetMathLibrary.MakeTransform` (- _returnvalue_location (`KismetMathLibrary.MakeVector` 0.0 Y)) _returnvalue_rotation _returnvalue_scale) false false)
  (`SceneComponent.K2_SetWorldLocation` (`Actor.RootComponent` (`self.Chair`)) (- (`SceneComponent.K2_GetComponentLocation` (`Actor.RootComponent` (`self.Chair`))) (`KismetMathLibrary.MakeVector` 0.0 Y)) false false))

(fn `DecreaseKPI`
  (params (DecreaseAmount :type Integer))
  (bind _output_get (set `self.ProductivityScore` (- (`self.ProductivityScore`) DecreaseAmount)))
  (`self.SetProductivityScore` _output_get))

(fn `GetBackToWork`
  (bind _output_get (set `self.CurrentState` "NewEnumerator1"))
  (`BlackboardComponent.SetValueAsEnum` (`AIBlueprintHelperLibrary.GetBlackboard` null) "CurrentState" _output_get)
  (`self.MoveChairForwardEvent`)
  (`SceneComponent.SetHiddenInGame` (`self.Niagara`) true false))

(fn `MoveChairBackward`
  (params (Alpha :type "Float (single-precision)"))
  (bind _chair (`self.Chair`))
  (`SceneComponent.K2_SetWorldLocation` (`/Game/Blueprints/BP_Chair.StaticMesh` (`self.Chair`)) (`KismetMathLibrary.VLerp` (`SceneComponent.K2_GetComponentLocation` (`/Game/Blueprints/BP_Chair.ForwardPoint` _chair)) (`SceneComponent.K2_GetComponentLocation` (`/Game/Blueprints/BP_Chair.BackwardPoint` _chair)) Alpha) false false))

(fn `MoveChairFoward`
  (params (Alpha :type "Float (single-precision)"))
  (bind _chair (`self.Chair`))
  (`SceneComponent.K2_SetWorldLocation` (`/Game/Blueprints/BP_Chair.StaticMesh` (`self.Chair`)) (`KismetMathLibrary.VLerp` (`SceneComponent.K2_GetComponentLocation` (`/Game/Blueprints/BP_Chair.BackwardPoint` _chair)) (`SceneComponent.K2_GetComponentLocation` (`/Game/Blueprints/BP_Chair.ForwardPoint` _chair)) Alpha) false false))

(fn `MoveEmployeeBackward`
  (params (yValue :type "Float (single-precision)"))
  (`SceneComponent.K2_SetWorldLocation` (`self.Mesh`) (`KismetMathLibrary.VLerp` (`SceneComponent.K2_GetComponentLocation` (`self.ForwardPoint`)) (`SceneComponent.K2_GetComponentLocation` (`self.BackWardPoint`)) yValue) false false))

(fn `MoveEmployeeForward`
  (params (yValue :type "Float (single-precision)"))
  (`SceneComponent.K2_SetWorldLocation` (`self.Mesh`) (`KismetMathLibrary.VLerp` (`SceneComponent.K2_GetComponentLocation` (`self.BackWardPoint`)) (`SceneComponent.K2_GetComponentLocation` (`self.ForwardPoint`)) yValue) false false))

(fn `MoveEmployeeForward2`
  (params (yValue :type "Float (single-precision)"))
  (`SceneComponent.K2_SetWorldLocation` (`self.Mesh`) (`KismetMathLibrary.VLerp` (`SceneComponent.K2_GetComponentLocation` (`self.BackWardPoint`)) (`SceneComponent.K2_GetComponentLocation` (`self.ForwardPoint`)) yValue) false false))

(fn `NewFunction`)

(fn `ResetStates`
  (bind _computer (`self.Computer`))
  (bind _bp_phone (`self.BP_Phone`)
    (:`then`
      (`self.K2_DestroyActor` _bp_phone))
    (:`else`
      _))
  (`SceneComponent.SetHiddenInGame` (`self.Niagara`) true false)
  (if (not (`SceneComponent.bHiddenInGame` (`/Game/Blueprints/BP_Computer.Niagara` _computer)))
    (`/Game/Blueprints/BP_Computer.SwitchComputerOverloading` _computer)))

(fn `SetCircle`
  (params (CircleScale :type "Vector Structure"))
  (`SceneComponent.SetWorldScale3D` (`self.Plane`) CircleScale))

(fn `SetProductivityScore`
  (params (TargetProductivityScore :type Integer))
  (bind (_returnvalue_location _returnvalue_rotation) (`KismetMathLibrary.BreakTransform` (`self.GetTransform` (`GameplayStatics.GetPlayerCameraManager` 0))))
  (`TextRenderComponent.K2_SetText` (`self.ProductScore`) (`KismetTextLibrary.Conv_IntToText` TargetProductivityScore))
  (`SceneComponent.K2_SetWorldRotation` (`self.ProductScore`) _returnvalue_rotation false false)
  (`SceneComponent.K2_AddWorldRotation` (`self.ProductScore`) (struct :`Yaw` 180.0) false false))

(fn `UpdatingProductivityScore`
  (bind _productscore (`self.ProductScore`))
  (bind (_returnvalue_location _returnvalue_rotation) (`KismetMathLibrary.BreakTransform` (`self.GetTransform` (`GameplayStatics.GetPlayerCameraManager` 0))))
  (bind _output_get (set `self.ProductivityScore` (+ (`self.ProductivityScore`) (`self.ProductivityIncreaseRate`))))
  (`TextRenderComponent.K2_SetText` (`self.ProductScore`) (`KismetTextLibrary.Conv_IntToText` _output_get))
  (`SceneComponent.K2_SetWorldRotation` _productscore _returnvalue_rotation false false)
  (`SceneComponent.K2_AddLocalRotation` _productscore (struct :`Yaw` 180.0) false false))

(fn `UserConstructionScript`)