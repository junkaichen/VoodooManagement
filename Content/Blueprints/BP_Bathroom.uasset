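; Bathroom trigger actor that tells an AI-driven BP_TESTING character it has entered the bathroom.
; When one overlaps the Box component, it writes the IsInBathRoom flag to that character's Blackboard.
; It also sets BathRoomTime there, with a longer time for the I Walking state than for C Walking.
; The actor only writes on begin overlap and never clears the flag itself.
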(event `self.ReceiveTick`
  (params (DeltaSeconds :type "Float (single-precision)")))

(event `self.Box.OnComponentBeginOverlap`
  (params (OverlappedComponent :type "PrimitiveComponent Object Reference") (OtherActor :type "Actor Object Reference") (OtherComp :type "PrimitiveComponent Object Reference") (OtherBodyIndex :type Integer) (bFromSweep :type Boolean) (SweepResult :type "HitResult Structure (by ref)"))
  (bind _asbp_testing (cast `/Game/Blueprints/BP_TESTING` OtherActor))
  (`BlackboardComponent.SetValueAsBool` (`AIBlueprintHelperLibrary.GetBlackboard` _asbp_testing) "IsInBathRoom" true)
  (switch `/Game/EmployeeStates` (`/Game/Blueprints/BP_TESTING.CurrentState` _asbp_testing)
    (:`NewEnumerator0`
      (`BlackboardComponent.SetValueAsFloat` (`AIBlueprintHelperLibrary.GetBlackboard` _asbp_testing) "BathRoomTime" 5.0))
    (:`NewEnumerator4`
      (`BlackboardComponent.SetValueAsFloat` (`AIBlueprintHelperLibrary.GetBlackboard` _asbp_testing) "BathRoomTime" 10.0))))

(fn `UserConstructionScript`)