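; Test Blueprint for an office employee who sits at an assigned chair and switches between walking, working, phone use and sleeping.
; Chair overlap seats the employee working; the self-looping RandomState event picks later states, driving timeline chair/body lerps, audio and a phone prop.
; Working raises a camera-facing productivity score, and Pined overrides state, slides the employee forward, then restores working.
; Walking and seating update the Blackboard; EndPlay closes the Arduino port.
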(event `self.ReceiveBeginPlay`)

(event `self.ReceiveEndPlay`
  (params (EndPlayReason :type "EEndPlayReason Enum" :default "Destroyed"))
  (bind _ardurio (`self.Ardurio`))
  ;[1 1 1] GameEnd Close Arduino Portal
  (`/Engine/EditorBlueprintResources/StandardMacros.IsValid` _ardurio
    (:`Is Valid`
      (`SerialCom.Close` _ardurio))))

(event `RandomState`
  (bind _audio (`self.Audio`))
  (bind _audio_2 (`self.Audio`))
  (bind _audio_3 (`self.Audio`))
  (if (`|EnumInequality` (`self.CurrentState`) "NewEnumerator0")
    (`KismetSystemLibrary.Delay` (`KismetMathLibrary.RandomFloatInRange` 5.0 10.0))
    (bind _bp_phone (`self.BP_Phone`)
      (:`then`
        (`self.K2_DestroyActor` _bp_phone))
      (:`else`
        _))
    (bind _output_get (set `self.CurrentState` (cast `/Game/EmployeeStates` (`KismetMathLibrary.Conv_IntToByte` (`KismetMathLibrary.RandomIntegerInRange` 0 3)))))
    (if (`|EnumEquality` _output_get "NewEnumerator0")
      (`AudioComponent.Stop` (`self.Audio`))
      ;[1 1 1] Walking
      (bind (_direction _movechairtime) (`Timeline|Timeline` :!via `PlayFromStart`)
        (:`Update`
          (if (`self.IsForward`)
            (`self.MoveChairBackward` _movechairtime)
            (`self.MoveEmployeeBackward` _movechairtime)))
        (:`Finished`
          (`SceneComponent.K2_SetRelativeTransform` (`self.Mesh`) (`self.NewVar`) false false)
          (`SceneComponent.K2_SetRelativeTransform` (`self.ChairPoint`) (`self.NewVar`) false false)
          (`SceneComponent.K2_SetRelativeTransform` (`self.Mesh`) (`self.MeshStartTransform`) false false)
          (`BlackboardComponent.SetValueAsEnum` (`AIBlueprintHelperLibrary.GetBlackboard` null) "CurrentState" (`self.CurrentState`))
          (set `self.IsForward` false)
          (`self.RandomState`)))
      (else
        ;[1 1 1] PlayingCellPhone
        (if (`|EnumEquality` (`self.CurrentState`) "NewEnumerator3")
          (bind (_direction_2 _movechairtime_2) (`Timeline|Timeline_0` :!via `PlayFromStart`)
            (:`Update`
              (if (`self.IsForward`)
                (`self.MoveChairBackward` _movechairtime_2)
                (`self.MoveEmployeeBackward` _movechairtime_2)))
            (:`Finished`
              (bind _returnvalue (`|SpawnActorFromClass` "/Game/Blueprints/AnimatedItems/BP_Phone.BP_Phone_C" (`KismetMathLibrary.MakeTransform` (0.0 0.0 0.0)) "Undefined" "OverrideRootScale" null self))
              (bind _output_get_2 (set `self.BP_Phone` _returnvalue))
              (`SceneComponent.K2_AttachToComponent` (`Actor.RootComponent` _output_get_2) (`self.Mesh`) "RightHandSocket" "KeepRelative" "KeepRelative" "KeepRelative" true)
              (set `self.IsForward` false)
              (`AudioComponent.SetSound` _audio_2 "/Game/Audio/PhoneTyping_01.PhoneTyping_01")
              (`AudioComponent.Play` _audio_2 0.0)
              (`self.RandomState`)))
          (else
            ;[1 1 1] Sleeping
            (if (`|EnumEquality` (`self.CurrentState`) "NewEnumerator2")
              (bind (_direction_3 _movechairtime_3) (`Timeline|Timeline_3` :!via `PlayFromStart`)
                (:`Update`
                  (if (`self.IsForward`)
                    (`self.MoveChairBackward` _movechairtime_3)
                    (`self.MoveEmployeeBackward` _movechairtime_3)))
                (:`Finished`
                  (set `self.IsForward` false)
                  (`AudioComponent.SetSound` _audio "/Game/Audio/Snore.Snore")
                  (`AudioComponent.Play` _audio 0.0)
                  (`self.RandomState`)))
              (else
                ;[1 1 1] Working
                (if (`|EnumEquality` (`self.CurrentState`) "NewEnumerator1")
                  (bind (_direction_4 _movechairtime_4) (`Timeline|Timeline_4` :!via `PlayFromStart`)
                    (:`Update`
                      (if (not (`self.IsForward`))
                        (`self.MoveChairFoward` _movechairtime_4)
                        (`self.MoveEmployeeForward` _movechairtime_4)))
                    (:`Finished`
                      (set `self.IsForward` true)
                      (`AudioComponent.SetSound` _audio_3 "/Game/Audio/Keyboard_01.Keyboard_01")
                      (`AudioComponent.Play` _audio_3 0.0)
                      (`self.RandomState`))))))))))
    (else
      (`KismetSystemLibrary.Delay` 0.5)
      (`self.RandomState`))))

(event `self.ReceiveTick`
  (params (DeltaSeconds :type "Float (single-precision)"))
  (if (`|EnumEquality` (`self.CurrentState`) "NewEnumerator1")
    (`KismetSystemLibrary.Delay` 0.3)
    (`self.UpdatingProductivityScore`)))

(event `Pined`
  (params (EmployeeState :type "/Game/EmployeeStates Enum" :default "NewEnumerator0"))
  (bind _audio (`self.Audio`))
  (bind _output_get (set `self.CurrentState` EmployeeState))
  (`BlackboardComponent.SetValueAsEnum` (`AIBlueprintHelperLibrary.GetBlackboard` null) "CurrentState" _output_get)
  (bind (_direction _movechairtime) (`Timeline|Timeline_1` :!via `PlayFromStart`)
    (:`Update`
      (`self.MoveChairFoward` _movechairtime)
      (`self.MoveEmployeeForward` _movechairtime)
      (`AudioComponent.SetSound` _audio "/Game/Audio/Keyboard_01.Keyboard_01")
      (`AudioComponent.Play` _audio 0.0)
      (set `self.IsForward` true)
      (`KismetSystemLibrary.Delay` 4.0)
      (set `self.CurrentState` "NewEnumerator1"))))

(event `self.CapsuleComponent.OnComponentBeginOverlap`
  (params (OverlappedComponent :type "PrimitiveComponent Object Reference") (OtherActor :type "Actor Object Reference") (OtherComp :type "PrimitiveComponent Object Reference") (OtherBodyIndex :type Integer) (bFromSweep :type Boolean) (SweepResult :type "HitResult Structure (by ref)"))
  (bind _chair (`self.Chair`))
  (bind _chairpoint (`self.ChairPoint`))
  (bind _mesh (`self.Mesh`))
  (bind _audio (`self.Audio`))
  (bind (_returnvalue_location _returnvalue_rotation) (`KismetMathLibrary.BreakTransform` (`SceneComponent.K2_GetComponentToWorld` (`/Game/Blueprints/BP_Chair.SitPosition` _chair))))
  (bind _asbp_chair (cast `/Game/Blueprints/BP_Chair` OtherActor))
  (if (== _asbp_chair _chair)
    (`SceneComponent.K2_SetWorldLocation` _chairpoint _returnvalue_location false false)
    (`SceneComponent.K2_SetWorldRotation` _chairpoint _returnvalue_rotation false false)
    (`SceneComponent.K2_SetWorldLocation` _mesh _returnvalue_location false false)
    (`SceneComponent.K2_SetWorldRotation` _mesh _returnvalue_rotation false false)
    (bind _output_get (set `self.CurrentState` "NewEnumerator1"))
    (`BlackboardComponent.SetValueAsEnum` (`AIBlueprintHelperLibrary.GetBlackboard` null) "CurrentState" _output_get)
    (bind (_direction _movechairtime) (`Timeline|Timeline_2` :!via `PlayFromStart`)
      (:`Update`
        (`self.MoveChairFoward` _movechairtime)
        (`self.MoveEmployeeForward2` _movechairtime))
      (:`Finished`
        (set `self.IsForward` true)
        (`AudioComponent.SetSound` _audio "/Game/Audio/Keyboard_01.Keyboard_01")
        (`AudioComponent.Play` _audio 0.0)))))

(fn `BackWardDesk`
  (params (Y :type "Float (single-precision)"))
  (bind (_returnvalue_location _returnvalue_rotation _returnvalue_scale) (`KismetMathLibrary.BreakTransform` (`SceneComponent.K2_GetComponentToWorld` (`self.Mesh`))))
  (`SceneComponent.K2_SetWorldTransform` (`self.Mesh`) (`KismetMathLibrary.MakeTransform` (- _returnvalue_location (`KismetMathLibrary.MakeVector` 0.0 Y)) _returnvalue_rotation _returnvalue_scale) false false)
  (`SceneComponent.K2_SetWorldLocation` (`Actor.RootComponent` (`self.Chair`)) (- (`SceneComponent.K2_GetComponentLocation` (`Actor.RootComponent` (`self.Chair`))) (`KismetMathLibrary.MakeVector` 0.0 Y)) false false))

(fn `MoveChairBackward`
  (params (Alpha :type "Float (single-precision)"))
  (bind _chair (`self.Chair`))
  (`SceneComponent.K2_SetWorldLocation` (`/Game/Blueprints/BP_Chair.StaticMesh` (`self.Chair`)) (`KismetMathLibrary.VLerp` (`SceneComponent.K2_GetComponentLocation` (`/Game/Blueprints/BP_Chair.ForwardPoint` _chair)) (`SceneComponent.K2_GetComponentLocation` (`/Game/Blueprints/BP_Chair.BackwardPoint` _chair)) Alpha) false false))

(fn `MoveChairFoward`
  (params (Alpha :type "Float (single-precision)"))
  (bind _chair (`self.Chair`))
  (`SceneComponent.K2_SetWorldLocation` (`/Game/Blueprints/BP_Chair.StaticMesh` (`self.Chair`)) (`KismetMathLibrary.VLerp` (`SceneComponent.K2_GetComponentLocation` (`/Game/Blueprints/BP_Chair.BackwardPoint` _chair)) (`SceneComponent.K2_GetComponentLocation` (`/Game/Blueprints/BP_Chair.ForwardPoint` _chair)) Alpha) false false))

(fn `MoveEmployeeBackward`
  (params (yValue :type "Float (single-precision)"))
  (`SceneComponent.K2_SetWorldLocation` (`self.Mesh`) (`KismetMathLibrary.VLerp` (`SceneComponent.K2_GetComponentLocation` (`self.ForwardPoint`)) (`SceneComponent.K2_GetComponentLocation` (`self.BackWardPoint`)) yValue) false false))

(fn `MoveEmployeeForward`
  (params (yValue :type "Float (single-precision)"))
  (`SceneComponent.K2_SetWorldLocation` (`self.Mesh`) (`KismetMathLibrary.VLerp` (`SceneComponent.K2_GetComponentLocation` (`self.BackWardPoint`)) (`SceneComponent.K2_GetComponentLocation` (`self.ForwardPoint`)) yValue) false false))

(fn `MoveEmployeeForward2`
  (params (yValue :type "Float (single-precision)"))
  (`SceneComponent.K2_SetWorldLocation` (`self.Mesh`) (`KismetMathLibrary.VLerp` (`SceneComponent.K2_GetComponentLocation` (`self.BackWardPoint`)) (`SceneComponent.K2_GetComponentLocation` (`self.ForwardPoint`)) yValue) false false))

(fn `SetCircle`
  (params (CircleScale :type "Vector Structure"))
  (`SceneComponent.SetWorldScale3D` (`self.Plane`) CircleScale))

(fn `SetProductivityScore`
  (params (TargetProductivityScore :type Integer))
  (bind (_returnvalue_location _returnvalue_rotation) (`KismetMathLibrary.BreakTransform` (`self.GetTransform` (`GameplayStatics.GetPlayerCameraManager` 0))))
  (`TextRenderComponent.K2_SetText` (`self.ProductScore`) (`KismetTextLibrary.Conv_IntToText` TargetProductivityScore))
  (`SceneComponent.K2_SetWorldRotation` (`self.ProductScore`) _returnvalue_rotation false false)
  (`SceneComponent.K2_AddWorldRotation` (`self.ProductScore`) (struct :`Yaw` 180.0) false false))

(fn `UpdatingProductivityScore`
  (bind _productscore (`self.ProductScore`))
  (bind (_returnvalue_location _returnvalue_rotation) (`KismetMathLibrary.BreakTransform` (`self.GetTransform` (`GameplayStatics.GetPlayerCameraManager` 0))))
  (bind _output_get (set `self.ProductivityScore` (+ (`self.ProductivityScore`) 1)))
  (`TextRenderComponent.K2_SetText` (`self.ProductScore`) (`KismetTextLibrary.Conv_IntToText` _output_get))
  (`SceneComponent.K2_SetWorldRotation` _productscore _returnvalue_rotation false false)
  (`SceneComponent.K2_AddLocalRotation` _productscore (struct :`Yaw` 180.0) false false))

(fn `UserConstructionScript`)