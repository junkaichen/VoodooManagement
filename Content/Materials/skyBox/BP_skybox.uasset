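; BP_skybox is a day/night cycle actor that rotates a directional light and swaps the sky sphere's material.
; Each Tick that passes the Timer/TimeLength check advances the light's pitch by CircleSpeed scaled by delta time and zeroes Timer.
; When the rotation nears either of two target angles, it applies the day or night material through paired DoOnce gates that reset each other, so each swap fires once per crossing.
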(event `self.ReceiveTick`
  (params (DeltaSeconds :type "Float (single-precision)"))
  (bind _directionallight (`self.DirectionalLight`))
  (bind _returnvalue (`self.K2_GetActorRotation` _directionallight))
  (bind (_returnvalue_roll _returnvalue_pitch) (`KismetMathLibrary.BreakRotator` (`self.K2_GetActorRotation` (`self.DirectionalLight`))))
  (bind _staticmeshcomponent (`StaticMeshActor.StaticMeshComponent` (`self.skySphere`)))
  (if (>= (`self.timeLength`) (+ DeltaSeconds (`self.timer`)))
    (`/Engine/EditorBlueprintResources/StandardMacros.IsValid` _directionallight
      (:`Is Valid`
        (`self.K2_SetActorRotation` (`self.DirectionalLight`) (`KismetMathLibrary.MakeRotator` 0.0 (+ (* DeltaSeconds (`self.circleSpeed`)) _returnvalue_pitch)) false)
        (set `self.timer` 0.0)
        (`/Engine/EditorBlueprintResources/StandardMacros.IsValid` (`self.skySphere`)
          (:`Is Valid`
            (if (== _returnvalue (struct :`Yaw` 180.0 :`Roll` 180.0) :`ErrorTolerance` 1.0)
              (`/Engine/EditorBlueprintResources/StandardMacros.DoOnce` false :!label _label
                (:`Completed`
                  (`|ExecutionSequence`
                    (:`then_0`
                      (`PrimitiveComponent.SetMaterial` _staticmeshcomponent 0 "/Game/Materials/skyBox/sky_DAY.sky_DAY"))
                    (:`then_1`
                      (goto _label_2 :!via `Reset`)))))
              (elif (== _returnvalue (struct) :`ErrorTolerance` 1.0)
                (`/Engine/EditorBlueprintResources/StandardMacros.DoOnce` false :!label _label_2
                  (:`Completed`
                    (`|ExecutionSequence`
                      (:`then_0`
                        (goto _label :!via `Reset`))
                      (:`then_1`
                        (`PrimitiveComponent.SetMaterial` _staticmeshcomponent 0 "/Game/Materials/skyBox/sky_NIGHT.sky_NIGHT")))))))))))))

(fn `UserConstructionScript`)